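; Player controller Blueprint that owns the game's dialogue and HUD widgets.
; On BeginPlay it creates both widgets, stores references, adds them to the viewport and starts them hidden.
; Four custom events show or hide each widget independently by toggling its visibility, so they are never recreated.
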(event `self.ReceiveBeginPlay`
  (`|ExecutionSequence`
    (:`then_0`
      (bind _returnvalue (`|CreateWidget` "/Game/BP_Dialogue.BP_Dialogue_C" self))
      (bind _output_get (set `self.DialogueWidgetRef` _returnvalue))
      (`UserWidget.AddToViewport` _output_get 0)
      (`self.HideDialogueUI`))
    (:`then_1`
      (bind _returnvalue_2 (`|CreateWidget` "/Game/Blueprints/GUI/BP_HUD.BP_HUD_C" self))
      (bind _output_get_2 (set `self.HudRef` _returnvalue_2))
      (`UserWidget.AddToViewport` _output_get_2 0)
      (`self.HideHUD`))))

(event `ShowDialogueUI`
  (`Widget.SetVisibility` (`self.DialogueWidgetRef`) "Visible"))

(event `ShowHUD`
  (`Widget.SetVisibility` (`self.HudRef`) "Visible"))

(event `HideDialogueUI`
  (`Widget.SetVisibility` (`self.DialogueWidgetRef`) "Hidden"))

(event `HideHUD`
  (`Widget.SetVisibility` (`self.HudRef`) "Hidden"))

(fn `UserConstructionScript`)