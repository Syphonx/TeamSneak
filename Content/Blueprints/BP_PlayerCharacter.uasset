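; Player character Blueprint that handles talking to quest-giving villagers and detecting found items.
; Overlapping a villager stores it and toggles the interact HUD through the player controller.
; E queues that villager's quest dialogue in the dialogue UI, which Enter, Escape or ending the overlap closes.
; Each tick, a very short forward line trace from eye level stores any hit found item, though nothing here uses it.
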(event `self.ReceiveBeginPlay`
  (bind _asbp_player_controller (cast `/Game/Blueprints/BP_PlayerController` (`GameplayStatics.GetPlayerController` 0)))
  (set `self.PlayerControllerRef` _asbp_player_controller))

(event `self.ReceiveTick`
  (params (DeltaSeconds :type "Float (single-precision)"))
  (bind _outlocation (`self.GetActorEyesViewPoint`))
  (bind (_outhit _returnvalue) (`KismetSystemLibrary.LineTraceSingleForObjects` _outlocation (+ _outlocation (`self.GetActorForwardVector`)) (`self.ObjectTraceTypes`)))
  (if _returnvalue
    (bind _asbp_found_item (cast `/Game/Blueprints/BP_FoundItem` (`.HitActor` (`GameplayStatics.BreakHitResult` _outhit))))
    (set `self.CurrentItem` _asbp_found_item)
    (else
      (set `self.CurrentItem` null))))

(event `self.ReceiveActorBeginOverlap`
  (params (OtherActor :type "Actor Object Reference"))
  (bind _asbp_villager_pawn (cast `/Game/Blueprints/BP_VillagerPawn` OtherActor))
  (set `self.CurrentVillager` _asbp_villager_pawn)
  (`self.ShowInteractHUD`))

(event `self.ReceiveActorEndOverlap`
  (params (OtherActor :type "Actor Object Reference"))
  (cast `/Game/Blueprints/BP_VillagerPawn` OtherActor)
  (set `self.CurrentVillager` null)
  (`self.HideInteractHUD`)
  (`self.CloseDialogue`))

(event `Key|E`
  (params (Key :type "Key Structure"))
  (bind _playercontrollerref (`self.PlayerControllerRef`))
  (:`Pressed`
    (if (`self.bCanInteract`)
      (`/Game/Blueprints/BP_PlayerController.HideHUD` _playercontrollerref)
      (`/Game/Blueprints/BP_PlayerController.ShowDialogueUI` _playercontrollerref)
      (`/Game/BP_Dialogue.QueueText` (`/Game/Blueprints/BP_PlayerController.DialogueWidgetRef` _playercontrollerref) (`VillagerQuest.QuestDialogue` (`/Game/Blueprints/BP_VillagerPawn.Quest` (`self.CurrentVillager`))))
      (set `self.bInDialogue` true))))

(event `ShowInteractHUD`
  (bind _playercontrollerref (`self.PlayerControllerRef`))
  (`/Game/Blueprints/BP_PlayerController.ShowHUD` _playercontrollerref)
  (`/Game/Blueprints/GUI/BP_HUD.CanInteract` (`/Game/Blueprints/BP_PlayerController.HudRef` _playercontrollerref) true)
  (set `self.bCanInteract` true))

(event `Key|Enter`
  (params (Key :type "Key Structure"))
  (:`Pressed`
    (`self.CloseDialogue`)))

(event `Key|Escape`
  (params (Key :type "Key Structure"))
  (:`Pressed`
    (`self.CloseDialogue`)))

(event `HideInteractHUD`
  (bind _playercontrollerref (`self.PlayerControllerRef`))
  (`/Game/Blueprints/BP_PlayerController.HideHUD` _playercontrollerref)
  (`/Game/Blueprints/GUI/BP_HUD.CanInteract` (`/Game/Blueprints/BP_PlayerController.HudRef` _playercontrollerref) false)
  (set `self.bCanInteract` false))

(event `CloseDialogue`
  (bind _playercontrollerref (`self.PlayerControllerRef`))
  (if (`self.bInDialogue`)
    (`/Game/Blueprints/BP_PlayerController.HideDialogueUI` _playercontrollerref)
    (`/Game/Blueprints/BP_PlayerController.ShowHUD` _playercontrollerref)
    (set `self.bInDialogue` false)))

(fn `UserConstructionScript`)