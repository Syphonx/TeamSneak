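; Start screen actor that shows the intro widget over its own camera view, then hands the view to the player character.
; BeginPlay fades in and opens an initially closed DoOnce after ten seconds, so earlier key presses are ignored.
; Any key then fades out music and screen, quits the widget, switches view and disables its input.
; The LoopDeLoop timeline eases the camera along a spline, though no graph wire starts it.
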(event `Key|AnyKey`
  (params (Key :type "Key Structure"))
  (:`Pressed`
    (`/Engine/EditorBlueprintResources/StandardMacros.DoOnce` true :!label _label
      (:`Completed`
        (`AudioComponent.FadeOut` (`self.Lofi_beats_to_find_objects_to__intro_`) 2.0 0.0 "Linear")
        (`PlayerCameraManager.StartCameraFade` (`GameplayStatics.GetPlayerCameraManager` 0) 0.0 1.0 2.0 (struct :`R` 0.03125 :`G` 0.024521 :`B` 0.013149 :`A` 1.0) true false)
        (`/Game/Blueprints/W_IntroScreen.Quit` (`self.Start Screen`))
        (`KismetSystemLibrary.Delay` 2.0)
        (`PlayerController.SetViewTargetWithBlend` (`GameplayStatics.GetPlayerController` 0) (`GameplayStatics.GetPlayerCharacter` 0) 0.0 "VTBlend_Linear" 0.0 false)
        (`PlayerCameraManager.StartCameraFade` (`GameplayStatics.GetPlayerCameraManager` 0) 1.0 0.0 1.0 (struct :`R` 0.03125 :`G` 0.024521 :`B` 0.013149 :`A` 1.0) true false)
        (`self.DisableInput` (`GameplayStatics.GetPlayerController` 0))))))

(event `self.ReceiveBeginPlay`
  (bind _returnvalue (`GameplayStatics.GetPlayerController` 0))
  (`TimelineComponent.SetPlayRate` (`self.LoopDeLoop`) (/ 1.0 (`self.TimePerLoop`)))
  (`PlayerController.SetViewTargetWithBlend` (`GameplayStatics.GetPlayerController` 0) self 0.0 "VTBlend_Linear" 0.0 false)
  (`PlayerCameraManager.StartCameraFade` (`GameplayStatics.GetPlayerCameraManager` 0) 1.0 0.0 1.0 (struct :`R` 1.0 :`G` 0.784665 :`B` 0.420773 :`A` 1.0) false false)
  (`self.EnableInput` _returnvalue)
  (bind _returnvalue_2 (`|CreateWidget` "/Game/Blueprints/W_IntroScreen.W_IntroScreen_C" _returnvalue))
  (bind _output_get (set `self.Start Screen` _returnvalue_2))
  (`UserWidget.AddToViewport` _output_get 0)
  (`KismetSystemLibrary.Delay` 10.0)
  (goto _label :!via `Reset`))

(fn `UserConstructionScript`)