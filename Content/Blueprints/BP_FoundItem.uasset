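; BP_FoundItem is a world item pickup, shown as a billboard and configured through its ItemInfo data.
; On BeginPlay it creates a dynamic instance of the item's material, writes it into the first billboard element and applies the elements to ItemBillboard.
; The OnPickupItem event destroys the actor; overlap and Tick do nothing here, and a debug draw of the PickupRadius sphere is left unconnected.
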(event `self.ReceiveBeginPlay`
  (bind _returnvalue (`KismetMaterialLibrary.CreateDynamicMaterialInstance` (`ItemInfo.ItemMaterial` (`self.ItemInfo`))))
  (setmembers `MaterialSpriteElement` :`StructRef` (`|GetArrayItem` (`self.BillboardElement`)) :`Material` _returnvalue)
  (`MaterialBillboardComponent.SetElements` (`self.ItemBillboard`) (`self.BillboardElement`)))

(event `self.ReceiveTick`
  (params (DeltaSeconds :type "Float (single-precision)")))

(event `OnPickupItem`
  (`self.K2_DestroyActor`))

(fn `UserConstructionScript`)