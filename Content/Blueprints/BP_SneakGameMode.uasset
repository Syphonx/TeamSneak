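; Game mode for the sneak game that places one findable item per item type at a random matching spawn point when play begins.
; It gathers all BP_ItemSpawnLocation actors, then loops over the AllItemTypes map keys, spawning a BP_FoundItem with that type's ItemInfo.
; PickRandomSpawn rerolls random locations until the ItemType matches, so it never exits if a type has no matching spawn point.
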(event `self.ReceiveBeginPlay`
  (bind _allitemtypes (`self.AllItemTypes`))
  (`|ExecutionSequence`
    (:`then_0`
      (bind _outactors (`GameplayStatics.GetAllActorsOfClass` "/Game/Blueprints/BP_ItemSpawnLocation.BP_ItemSpawnLocation_C")) ; Find
      (set `self.SpawnedTypes` _outactors))
    (:`then_1`
      (bind _keys (`BlueprintMapLibrary.Map_Keys` _allitemtypes))
      (for (_array_element _array_index) _keys
        (bind _locationactor (`self.PickRandomSpawn` _array_element))
        (bind (_value _returnvalue) (`BlueprintMapLibrary.Map_Find` _allitemtypes (`|GetArrayItem` _keys _array_index)))
        (if _returnvalue
          (`|SpawnActorFromClass` "/Game/Blueprints/BP_FoundItem.BP_FoundItem_C" (`SceneComponent.K2_GetComponentToWorld` (`/Game/Blueprints/BP_ItemSpawnLocation.DefaultSceneRoot` _locationactor)) "Undefined" "OverrideRootScale" null _value null))))))

(fn `PickRandomSpawn`
  (params (SpawnType :type "EItemType Enum" :default "Hat"))
  (returns (LocationActor :type "/Game/Blueprints/BP_ItemSpawnLocation Object Reference"))
  (locals (bFound :type Boolean) (FoundActor :type "/Game/Blueprints/BP_ItemSpawnLocation Object Reference"))
  (bind _spawnedtypes (`self.SpawnedTypes`))
  (set `local.bFound` false)
  (while (not (`local.bFound`))
    (bind _output_get (set `local.FoundActor` (`|GetArrayItem` _spawnedtypes (`KismetMathLibrary.RandomIntegerInRange` 0 (- (`KismetArrayLibrary.Array_Length` _spawnedtypes) 1)))))
    (set `local.bFound` (`|EnumEquality` (`/Game/Blueprints/BP_ItemSpawnLocation.ItemType` _output_get) SpawnType)))
  (return (`local.FoundActor`)))

(fn `UserConstructionScript`)